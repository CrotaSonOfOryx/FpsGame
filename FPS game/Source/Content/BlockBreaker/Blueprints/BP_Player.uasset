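; BP_Player is the first-person player character for BlockBreaker, with movement, mouse look, jumping and shooting.
; On BeginPlay it spawns a BP_Riffle, stores it as the equipped gun and snaps it to the GunLocation component.
; Holding Shoot fires the gun along the camera's forward vector up to its max bullet distance, with a CanShoot flag and Delay enforcing the gun's fire rate.
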(event `InputAxis|Shoot`
  (params (AxisValue :type "Float (single-precision)"))
  (bind _fpscamera (`self.FpsCamera`))
  (bind _returnvalue (`SceneComponent.K2_GetComponentLocation` _fpscamera))
  (if (and (`self.CanShoot`) (== AxisValue 1.0))
    (`/Game/BlockBreaker/Blueprints/BP_BaseGun.Shoot` (`self.EquippedGun`) _returnvalue (+ (* (`/Game/BlockBreaker/Blueprints/BP_BaseGun.MaxBulletDistance` (`self.EquippedGun`)) (`SceneComponent.GetForwardVector` _fpscamera)) _returnvalue))
    (set `self.CanShoot` false)
    (`KismetSystemLibrary.Delay` (`/Game/BlockBreaker/Blueprints/BP_BaseGun.FireRate` (`self.EquippedGun`)))
    (set `self.CanShoot` true)))

(event `InputAction|PlayerJump`
  (params (Key :type "Key Structure"))
  (:`Pressed`
    (`self.Jump`)))

(event `self.ReceiveBeginPlay`
  (bind _returnvalue (`|SpawnActorFromClass` "/Game/BlockBreaker/Blueprints/BP_Riffle.BP_Riffle_C" (`KismetMathLibrary.MakeTransform` (0.0 0.0 0.0)) "Undefined" "OverrideRootScale" null null))
  (bind _output_get (set `self.EquippedGun` _returnvalue))
  (`self.K2_AttachToComponent` _output_get (`self.GunLocation`) "None" "SnapToTarget" "SnapToTarget" "KeepRelative" true))

(event `InputAxis|MoveForward`
  (params (AxisValue :type "Float (single-precision)"))
  (`self.AddMovementInput` (`self.GetActorForwardVector`) AxisValue))

(event `InputAxis|MoveRight`
  (params (AxisValue :type "Float (single-precision)"))
  (`self.AddMovementInput` (`self.GetActorRightVector`) AxisValue))

(event `InputAxis|LookHorizontal`
  (params (AxisValue :type "Float (single-precision)"))
  (`self.AddControllerYawInput` AxisValue))

(event `InputAxis|LookVeritcal`
  (params (AxisValue :type "Float (single-precision)"))
  (`self.AddControllerPitchInput` (* AxisValue -1.0)))

(fn `UserConstructionScript`)