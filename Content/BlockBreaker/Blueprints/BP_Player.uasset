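; First-person shooter player character with movement, hitscan-style firing, five swappable guns, HUD widgets and online session host/join keys.
; Firing delegates the shot to the equipped gun, applies damage, then handles ammo, effects, recoil and fire-rate gating.
; Lethal damage refills HP, teleports to a random fixed point and increments the player's own Kills.
; A 30-second delayed check on Kills can show another widget; camera pitch passes through update events.
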(event `CastWidget`
  (bind _returnvalue (`|CreateWidget` "/Game/BlockBreaker/UI/WinWidget.WinWidget_C"))
  (`UserWidget.AddToViewport` _returnvalue 0))

(event `ServerWidget`
  (`self.CastWidget`))

(event `ParticleServ`
  (`GameplayStatics.SpawnEmitterAtLocation` "/Game/BlockBreaker/ParticleSystems/PS_BulletImpact.PS_BulletImpact" (stale `RepFire` _location))
  (`GameplayStatics.PlaySoundAtLocation` "/Game/BlockBreaker/Downloaded/GunSound.GunSound" (`SceneComponent.K2_GetComponentLocation` (`self.FpsCamera`)) (struct) 1.0 1.0 0.0 null null null null))

(event `self.ReceiveAnyDamage`
  (params (Damage :type "Float (single-precision)") (DamageType :type "DamageType Object Reference") (InstigatedBy :type "Controller Object Reference") (DamageCauser :type "Actor Object Reference"))
  (set `self.CurrentHP` (`KismetMathLibrary.FTrunc` (- (`self.CurrentHP`) Damage)))
  (if (<= (`self.CurrentHP`) 0)
    (set `self.CurrentHP` (`self.MaxHP`))
    (set `self.Array` (`|MakeArray` (`KismetMathLibrary.MakeVector` 10000.0 0.0 100.0) (`KismetMathLibrary.MakeVector` 0.0 10000.0 100.0) (`KismetMathLibrary.MakeVector` 10000.0 10000.0 100.0) (`KismetMathLibrary.MakeVector` 0.0 0.0 100.0) (`KismetMathLibrary.MakeVector` 6900.0 6900.0 100.0)))
    (`self.K2_TeleportTo` (`|GetArrayItem` (`self.Array`) (`KismetMathLibrary.RandomIntegerInRange` 0 4)))
    (set `self.Kills` (+ (`self.Kills`) 1))))

(event `RepEffects`
  (bind _equippedgun (`self.EquippedGun`))
  (set `/Game/BlockBreaker/Blueprints/BP_BaseGun.CurrentAmmo` (- (`/Game/BlockBreaker/Blueprints/BP_BaseGun.CurrentAmmo` _equippedgun) 1.0) _equippedgun)
  (`self.ParticleServ`)
  (`self.AddControllerPitchInput` (* (`/Game/BlockBreaker/Blueprints/BP_BaseGun.RecoilStr` (`self.EquippedGun`)) -1.0))
  (`self.RepShhot2`))

(event `RepFire`
  (bind _fpscamera (`self.FpsCamera`))
  (bind _equippedgun (`self.EquippedGun`))
  (bind _returnvalue (`SceneComponent.K2_GetComponentLocation` _fpscamera))
  (bind (_location _actor) (`/Game/BlockBreaker/Blueprints/BP_BaseGun.Shoot` _equippedgun _returnvalue (+ (* (`/Game/BlockBreaker/Blueprints/BP_BaseGun.MaxBulletDistance` (`self.EquippedGun`)) (`SceneComponent.GetForwardVector` _fpscamera)) _returnvalue) self))
  (`GameplayStatics.ApplyDamage` _actor (`/Game/BlockBreaker/Blueprints/BP_BaseGun.Damage` _equippedgun))
  (`self.RepEffects`))

(event `InputAxis|Shoot`
  (params (AxisValue :type "Float (single-precision)"))
  (if (and (!= (`/Game/BlockBreaker/Blueprints/BP_BaseGun.CurrentAmmo` (`self.EquippedGun`)) 0.0) (and (`self.CanShoot`) (== AxisValue 1.0)) true)
    (`self.RepFire`)))

(event `RepShhot2`
  (set `self.CanShoot` false)
  (`KismetSystemLibrary.Delay` (`/Game/BlockBreaker/Blueprints/BP_BaseGun.FireRate` (`self.EquippedGun`)))
  (set `self.CanShoot` true))

(event `InputAction|PlayerJump`
  (params (Key :type "Key Structure"))
  (:`Pressed`
    (`self.Jump`)))

(event `self.ReceiveBeginPlay`
  (bind _equippedgun (`self.EquippedGun`))
  (`|ExecutionSequence`
    (:`then_0`
      (bind _returnvalue (`|SpawnActorFromClass` "/Game/BlockBreaker/Blueprints/BP_Riffle.BP_Riffle_C" (`KismetMathLibrary.MakeTransform` (0.0 0.0 0.0)) "Undefined" "OverrideRootScale" null null))
      (bind _output_get (set `self.EquippedGun` _returnvalue))
      (`self.K2_AttachToComponent` _output_get (`self.GunLocation`) "None" "SnapToTarget" "SnapToTarget" "KeepRelative" true)
      (set `/Game/BlockBreaker/Blueprints/BP_BaseGun.CurrentAmmo` (`/Game/BlockBreaker/Blueprints/BP_BaseGun.MagSize` _equippedgun) _equippedgun))
    (:`then_1`
      (bind _returnvalue_2 (`|CreateWidget` "/Game/BlockBreaker/UI/AmmoWidget.AmmoWidget_C"))
      (bind _output_get_2 (set `self.AmmoWigget` _returnvalue_2))
      (`UserWidget.AddToViewport` _output_get_2 0))
    (:`then_2`
      (bind _returnvalue_3 (`|CreateWidget` "/Game/BlockBreaker/UI/HPWidget.HPWidget_C"))
      (bind _output_get_3 (set `self.HPWidget` _returnvalue_3))
      (`UserWidget.AddToViewport` _output_get_3 0))
    (:`then_3`
      (`KismetSystemLibrary.Delay` 30.0)
      (if (== (`self.Kills`) 0)
        (`self.ServerWidget`)
        (else
          (`KismetSystemLibrary.K2_SetTimer` null "delay" 3.0)
          (if (== (`self.Kills`) 1)
            (`self.ServerWidget`)
            (else
              (`KismetSystemLibrary.K2_SetTimer` null "delay" 3.0)
              (if (== (`self.Kills`) 0)
                (`self.ServerWidget`)
                (else
                  (`KismetSystemLibrary.K2_SetTimer` null "delay" 3.0)
                  (if (== (`self.Kills`) 2)
                    (`self.ServerWidget`)
                    (else
                      (`KismetSystemLibrary.K2_SetTimer` null "delay" 3.0)
                      (if (== (`self.Kills`) 3)
                        (`self.ServerWidget`)
                        (else
                          (`KismetSystemLibrary.K2_SetTimer` null "delay" 3.0)
                          (if (== (`self.Kills`) 5)
                            (`self.ServerWidget`)))))))))))))))

(event `InputAxis|MoveForward`
  (params (AxisValue :type "Float (single-precision)"))
  (`self.AddMovementInput` (`self.GetActorForwardVector`) AxisValue))

(event `InputAxis|MoveRight`
  (params (AxisValue :type "Float (single-precision)"))
  (`self.AddMovementInput` (`self.GetActorRightVector`) AxisValue))

(event `InputAxis|LookHorizontal`
  (params (AxisValue :type "Float (single-precision)"))
  (`self.AddControllerYawInput` AxisValue))

(event `InputAxis|LookVeritcal`
  (params (AxisValue :type "Float (single-precision)"))
  (`self.AddControllerPitchInput` (* AxisValue -1.0))
  (`self.EventUpdateCameraToServer` (`self.GetBaseAimRotation`)))

(event `InputAction|Reload`
  (params (Key :type "Key Structure"))
  (:`Pressed`
    (set `self.CanShoot` false)
    (`KismetSystemLibrary.Delay` (`/Game/BlockBreaker/Blueprints/BP_BaseGun.ReloadTime` (`self.EquippedGun`)))
    (`/Game/BlockBreaker/Blueprints/BP_BaseGun.Reload` (`self.EquippedGun`))
    (set `self.CanShoot` true)))

(event `Key|One`
  (params (Key :type "Key Structure"))
  (:`Pressed`
    (`self.K2_DestroyActor` (`self.EquippedGun`))
    (bind _returnvalue (`|SpawnActorFromClass` "/Game/BlockBreaker/Blueprints/BP_Riffle.BP_Riffle_C" (`KismetMathLibrary.MakeTransform` (0.0 0.0 0.0)) "Undefined" "OverrideRootScale" null null))
    (bind _output_get (set `self.EquippedGun` _returnvalue))
    (`self.K2_AttachToComponent` _output_get (`self.GunLocation`) "None" "SnapToTarget" "SnapToTarget" "KeepRelative" true)
    (set `/Game/BlockBreaker/Blueprints/BP_BaseGun.CurrentAmmo` 0.0 (`self.EquippedGun`))))

(event `Key|Two`
  (params (Key :type "Key Structure"))
  (:`Pressed`
    (`self.K2_DestroyActor` (`self.EquippedGun`))
    (bind _returnvalue (`|SpawnActorFromClass` "/Game/BlockBreaker/Blueprints/BP_Shotgun.BP_Shotgun_C" (`KismetMathLibrary.MakeTransform` (0.0 0.0 0.0)) "Undefined" "OverrideRootScale" null null))
    (bind _output_get (set `self.EquippedGun` _returnvalue))
    (`self.K2_AttachToComponent` _output_get (`self.GunLocation`) "None" "SnapToTarget" "SnapToTarget" "KeepRelative" true)
    (set `/Game/BlockBreaker/Blueprints/BP_BaseGun.CurrentAmmo` 0.0 (`self.EquippedGun`))))

(event `Key|Three`
  (params (Key :type "Key Structure"))
  (:`Pressed`
    (`self.K2_DestroyActor` (`self.EquippedGun`))
    (bind _returnvalue (`|SpawnActorFromClass` "/Game/BlockBreaker/Blueprints/BP_Sniper.BP_Sniper_C" (`KismetMathLibrary.MakeTransform` (0.0 0.0 0.0)) "Undefined" "OverrideRootScale" null null))
    (bind _output_get (set `self.EquippedGun` _returnvalue))
    (`self.K2_AttachToComponent` _output_get (`self.GunLocation`) "None" "SnapToTarget" "SnapToTarget" "KeepRelative" true)
    (set `/Game/BlockBreaker/Blueprints/BP_BaseGun.CurrentAmmo` 0.0 (`self.EquippedGun`))))

(event `Gun3`)

(event `Key|Four`
  (params (Key :type "Key Structure"))
  (:`Pressed`
    (`self.K2_DestroyActor` (`self.EquippedGun`))
    (bind _returnvalue (`|SpawnActorFromClass` "/Game/BlockBreaker/Blueprints/BP_Smg.BP_Smg_C" (`KismetMathLibrary.MakeTransform` (0.0 0.0 0.0)) "Undefined" "OverrideRootScale" null null))
    (bind _output_get (set `self.EquippedGun` _returnvalue))
    (`self.K2_AttachToComponent` _output_get (`self.GunLocation`) "None" "SnapToTarget" "SnapToTarget" "KeepRelative" true)
    (set `/Game/BlockBreaker/Blueprints/BP_BaseGun.CurrentAmmo` 0.0 (`self.EquippedGun`))))

(event `Key|Five`
  (params (Key :type "Key Structure"))
  (bind _equippedgun (`self.EquippedGun`))
  (:`Pressed`
    (`self.K2_DestroyActor` (`self.EquippedGun`))
    (bind _returnvalue (`|SpawnActorFromClass` "/Game/BlockBreaker/Blueprints/BP_Pistol.BP_Pistol_C" (`KismetMathLibrary.MakeTransform` (0.0 0.0 0.0)) "Undefined" "OverrideRootScale" null null))
    (bind _output_get (set `self.EquippedGun` _returnvalue))
    (`self.K2_AttachToComponent` _output_get (`self.GunLocation`) "None" "SnapToTarget" "SnapToTarget" "KeepRelative" true)
    (set `/Game/BlockBreaker/Blueprints/BP_BaseGun.CurrentAmmo` (`/Game/BlockBreaker/Blueprints/BP_BaseGun.MagSize` _equippedgun) _equippedgun)))

(event `EventUpdateCameraToServer`
  (params (HeadRotation :type "Rotator Structure"))
  (`SceneComponent.K2_SetWorldRotation` (`self.FpsCamera`) HeadRotation false false)
  (set `self.Had Rot` HeadRotation)
  (`self.EventCam`))

(event `EventCam`
  (`SceneComponent.K2_SetWorldRotation` (`self.FpsCamera`) (`self.Had Rot`) false false))

(event `Key|C`
  (params (Key :type "Key Structure"))
  (:`Pressed`
    (bind _returnvalue (`|CreateWidget` "/Game/BlockBreaker/UI/MultiWidget.MultiWidget_C"))
    (bind _output_get (set `self.MultiWidget` _returnvalue))
    (`UserWidget.AddToViewport` _output_get 0)))

(event `Key|M`
  (params (Key :type "Key Structure"))
  (:`Pressed`
    (`Widget.RemoveFromParent` (stale `Key|C` _output_get))))

(event `Key|J`
  (params (Key :type "Key Structure"))
  (:`Pressed`
    (`CreateSessionCallbackProxy.CreateSession` (`GameplayStatics.GetPlayerController` 0) 5
      (:`OnSuccess`
        (`GameplayStatics.OpenLevel` "DefMap" true "?listen")))))

(event `Key|K`
  (params (Key :type "Key Structure"))
  (:`Pressed`
    (bind _results (`FindSessionsCallbackProxy.FindSessions` (`GameplayStatics.GetPlayerController` 0) 100)
      (:`OnSuccess`
        (`JoinSessionCallbackProxy.JoinSession` (`GameplayStatics.GetPlayerController` 0) (`|GetArrayItem` _results))))))

(fn `EventCamera`)

(fn `UserConstructionScript`)